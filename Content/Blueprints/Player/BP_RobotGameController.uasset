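; Player controller for a robot game that sets up the card deck and on-screen spawn bar at BeginPlay.
; TestWidget fills the deck with four identical placeholder cards, each using the base spawn decal.
; BeginPlay then creates the bar and four card slot widgets, showing one deck card in each and registering each slot.
; An unconnected debug snippet would project the first slot's card onto the world.
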(event Custom|TestWidget
  (bind _returnvalue (Game|ConstructObjectfromClass "/Game/Blueprints/CardSystem/BP_Card.BP_Card_C" "/Game/Blueprints/CardSystem/BP_SpawnDecalBase.BP_SpawnDecalBase_C" "/Game/ImportedPackages/MSPresets/M_MS_Glass_Material/Textures/Black.Black"))
  (bind _returnvalue_2 (Game|ConstructObjectfromClass "/Game/Blueprints/CardSystem/BP_Card.BP_Card_C" "/Game/Blueprints/CardSystem/BP_SpawnDecalBase.BP_SpawnDecalBase_C" "/Game/ImportedPackages/MSPresets/MSTextures/Black.Black"))
  (bind _returnvalue_3 (Game|ConstructObjectfromClass "/Game/Blueprints/CardSystem/BP_Card.BP_Card_C" "/Game/Blueprints/CardSystem/BP_SpawnDecalBase.BP_SpawnDecalBase_C" "/Game/ImportedPackages/MSPresets/M_MS_Glass_Material/Textures/Black.Black"))
  (bind _returnvalue_4 (Game|ConstructObjectfromClass "/Game/Blueprints/CardSystem/BP_Card.BP_Card_C" "/Game/Blueprints/CardSystem/BP_SpawnDecalBase.BP_SpawnDecalBase_C" "/Game/ImportedPackages/MSPresets/M_MS_Glass_Material/Textures/Black.Black"))
  (Class|RobotGamePlayerController|SetDeck (Utilities|Array|MakeArray _returnvalue_4 _returnvalue_3 _returnvalue_2 _returnvalue)))

(event EventBeginPlay
  ;[1 1 1] Create Spawn Bar
  ;;[1 1 1] Set Deck Here
  (CallFunction|TestWidget)
  (Variables|Default|GetSpawnBar
    (:then
      _)
    (:else
      (bind _returnvalue (UserInterface|CreateWidget "/Game/UserInterface/Widgets/WBP_SpawnBar.WBP_SpawnBar_C" self))
      (Variables|Default|SetSpawnBar _returnvalue)))
  (UserInterface|Viewport|AddtoViewport (Variables|Default|GetSpawnBar) 0)
  (for _index (range 0 3)
    (bind _returnvalue_2 (UserInterface|CreateWidget "/Game/UserInterface/Widgets/WBP_CardSlot.WBP_CardSlot_C" self _index))
    (bind _returnvalue_3 (Class|RobotGamePlayerController|GetDeck))
    (Class|CardSlotWidget|SetCardonDisplay _returnvalue_2 (Utilities|Array|Get(acopy) _returnvalue_3 _index))
    (Default|AddSlot (Variables|Default|GetSpawnBar) _returnvalue_2)
    (Class|RobotGamePlayerController|SetSlot _returnvalue_2)))

(event EventTick
  (params (DeltaSeconds :type Float%20%28single-precision%29)))

(fn ConstructionScript)