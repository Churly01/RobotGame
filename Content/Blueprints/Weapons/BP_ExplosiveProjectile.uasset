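; Explosive projectile that bursts on hit, dealing radial falloff damage around the impact point.
; On authority, a hit calls MulticastEmitter to spawn the explosion effect, then casts the owner to BP_RobotGameCharacter.
; A successful cast prints the owner's class, applies damage ignoring and crediting that character, then destroys the projectile.
; A failed cast leaves the projectile alive after the effect, with no damage dealt.
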(event Custom|MulticastEmitter
  (params (Location :type Vector))
  (Effects|SpawnEmitteratLocation "/Game/StarterContent/Particles/P_Explosion.P_Explosion" Location "0, 0, 0" "2.000000,2.000000,2.000000"))

(event EventBeginPlay
  (|CallParentFunction) ; This node is disabled and will not be called.\nDrag off pins to build functionality.
)

(event Collision|EventActorBeginOverlap
  (params (OtherActor :type Actor%20Object%20Reference)))

(event EventTick
  (params (DeltaSeconds :type Float%20%28single-precision%29)))

(event Collision|EventHit
  (params (MyComp :type Primitive%20Component%20Object%20Reference) (Other :type Actor%20Object%20Reference) (OtherComp :type Primitive%20Component%20Object%20Reference) (bSelfMoved :type Boolean) (HitLocation :type Vector :default "0, 0, 0") (HitNormal :type Vector :default "0, 0, 0") (NormalImpulse :type Vector :default "0, 0, 0") (Hit :type Hit%20Result%20Structure%20%28by%20ref%29))
  (bind _returnvalue (Class|WeaponProjectile|GetAreaDamage))
  (bind _returnvalue_2 (Components|GetOwner))
  (bind _damageradius (Variables|Default|GetDamageRadius))
  (Networking|SwitchHasAuthority
    (:Authority
      (CallFunction|MulticastEmitter HitLocation)
      (bind _asbp_robot_game_character (Utilities|Casting|CastToBP_RobotGameCharacter _returnvalue_2))
      (Development|PrintString (Utilities|GetClassDisplayName (Utilities|GetClass _returnvalue_2)))
      (Class|GameplayStatics|ApplyRadialDamagewithFalloff _returnvalue (* _returnvalue (Variables|Default|GetMinimumDamageParam)) (+ HitLocation "0.000000,0,10.000000") _damageradius (* _damageradius 3.0) 1.0 "/Script/RobotGame.ExplosionDamage" (Utilities|Array|MakeArray _asbp_robot_game_character) _asbp_robot_game_character (Pawn|GetController _asbp_robot_game_character) "ECC_Visibility")
      (Actor|DestroyActor))))

(fn ConstructionScript
  (|CallParentFunction))