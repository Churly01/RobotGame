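; BP_WeaponProjectileBase is a weapon projectile actor, named as a base class, that destroys itself five seconds after spawning.
; On hit, it spawns an ImpactField actor at the hit location.
; It also pushes physics-simulating components with an impulse at its own location, scaling its velocity unevenly per axis, with Y ten times stronger.
; The hit does not destroy the projectile, so only the timer removes it.
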(event EventBeginPlay
  (Utilities|FlowControl|Delay 5.0)
  (Actor|DestroyActor))

(event Collision|EventHit
  (params (MyComp :type Primitive%20Component%20Object%20Reference) (Other :type Actor%20Object%20Reference) (OtherComp :type Primitive%20Component%20Object%20Reference) (bSelfMoved :type Boolean) (HitLocation :type Vector :default "0, 0, 0") (HitNormal :type Vector :default "0, 0, 0") (NormalImpulse :type Vector :default "0, 0, 0") (Hit :type Hit%20Result%20Structure%20%28by%20ref%29))
  (Game|SpawnActorfromClass "/Game/GC_Destructibles/ImpactField.ImpactField_C" (Math|Conversions|ToTransform(Vector) HitLocation) "Undefined" 0 0)
  (if (Physics|IsSimulatingPhysics OtherComp "None")
    (Physics|AddImpulseatLocation OtherComp (* (Transformation|GetVelocity) "10000.000000,100000.000000,10000.000000") (Transformation|GetActorLocation) "None")))

(fn ConstructionScript)